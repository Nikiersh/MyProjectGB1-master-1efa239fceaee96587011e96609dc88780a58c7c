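; BP_Toilet is a damage dealer that works as an automatic turret, spawning an actor at its Arrow while something triggers its Box.
; Box begin and end overlap set and clear the Shot flag, with no filter on the overlapping actor.
; A looping one-second Delay from BeginPlay calls Fire, which, while Shot is set, spends one round from AMMOAC and spawns the Class variable's actor, ignoring collisions.
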(event OnComponentBeginOverlap(Box)
  (params (OverlappedComponent :type Primitive%20Component%20Object%20Reference) (OtherActor :type Actor%20Object%20Reference) (OtherComp :type Primitive%20Component%20Object%20Reference) (OtherBodyIndex :type Integer) (bFromSweep :type Boolean) (SweepResult :type Hit%20Result%20Structure%20%28by%20ref%29))
  (Variables|Default|SetShot true))

(event OnComponentEndOverlap(Box)
  (params (OverlappedComponent :type Primitive%20Component%20Object%20Reference) (OtherActor :type Actor%20Object%20Reference) (OtherComp :type Primitive%20Component%20Object%20Reference) (OtherBodyIndex :type Integer))
  (Variables|Default|SetShot false))

(event Custom|Fire
  (bind _ammo_ac (Variables|Default|GetAMMO_AC))
  (if (Variables|Default|GetShot)
    (if (Default|CheckAmmo _ammo_ac 1)
      (Default|SubstructAmmo _ammo_ac 1)
      (Game|SpawnActorfromClass (Variables|Default|GetClass) (Transformation|GetWorldTransform (Variables|Default|GetArrow)) "AlwaysSpawn" "MultiplyWithRoot" 0 0))))

(event EventBeginPlay
  (Utilities|FlowControl|Delay 1.0 :!label _label)
  (CallFunction|Fire)
  (goto _label))

(fn ConstructionScript)