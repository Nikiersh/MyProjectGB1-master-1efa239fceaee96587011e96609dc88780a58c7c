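; table1 is a damage-dealer actor that calls Fire on a repeating 1.5-second timer, built as a looping Delay from BeginPlay.
; A separate custom event, gated by the Shot flag, checks and subtracts one round through AMMOAC, then spawns an Ammo_base2 at the Arrow's transform.
; The graph does not define Fire or show a caller for that event, and the parent BeginPlay call is disabled.
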(event Custom|CustomEvent
  (bind _ammo_ac (Variables|Default|GetAMMO_AC))
  (if (Variables|Default|GetShot)
    (if (Default|CheckAmmo _ammo_ac 1)
      (Default|SubstructAmmo _ammo_ac 1)
      (Game|SpawnActorfromClass "/Game/BluePrints/DamageDealers/ammo_base2.ammo_base2_C" (Transformation|GetWorldTransform (Variables|Default|GetArrow)) "AlwaysSpawn" "MultiplyWithRoot" 0 0))))

(event Collision|EventActorBeginOverlap
  (params (OtherActor :type Actor%20Object%20Reference)))

(event EventTick
  (params (DeltaSeconds :type Float%20%28single-precision%29)))

(event EventBeginPlay
  (Utilities|FlowControl|Delay 1.5 :!label _label)
  (CallFunction|Fire)
  (goto _label))

(fn ConstructionScript
  (|CallParentFunction))